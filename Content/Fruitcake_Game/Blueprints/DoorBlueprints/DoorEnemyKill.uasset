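; A door actor that slides down open once all tagged enemies in the level are gone.
; Every Tick it counts MushroomEnemy and FlowerEnemy actors tagged "DoorEnemy" and, at zero, plays a timeline lerping the door mesh downward.
; A DoorOpened flag set on timeline update blocks retriggering, with a FlipFlop whose second branch reverses the timeline.
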(event `self.ReceiveTick`
  (params (DeltaSeconds :type "Float (single-precision)"))
  ;[1 1 1] Button and Door Animation
  ;[1 1 1] dont look at this please
  (bind _outactors (`GameplayStatics.GetAllActorsOfClassWithTag` "/Game/Fruitcake_Game/Enemies/MushroomEnemy.MushroomEnemy_C" "DoorEnemy"))
  (bind _outactors_2 (`GameplayStatics.GetAllActorsOfClassWithTag` "/Game/Fruitcake_Game/Enemies/FlowerEnemy.FlowerEnemy_C" "DoorEnemy"))
  (set `self.enemyAmount` (+ (`KismetArrayLibrary.Array_Length` _outactors_2) (`KismetArrayLibrary.Array_Length` _outactors)))
  (if (== (`self.enemyAmount`) 0)
    (if (not (`self.doorOpened`))
      (`/Engine/EditorBlueprintResources/StandardMacros.FlipFlop`
        (:`A`
          (bind (_direction _doortrack) (`Timeline|DoorTimeline` :!label _label)
            (:`Update`
              (`SceneComponent.K2_SetRelativeLocation` (`self.DoorMesh`) (`KismetMathLibrary.VLerp` (0.0 0.0 0.0) (0.0 0.0 -500.0) _doortrack) false false)
              (set `self.doorOpened` true))))
        (:`B`
          (goto _label :!via `Reverse`))))))

(fn `UserConstructionScript`)