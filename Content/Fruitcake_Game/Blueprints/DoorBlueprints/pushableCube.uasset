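; Pushable cube actor that binds to the ThirdPerson_PerspectiveSwitch character and moves while a key is held.
; The first overlap of its Box with that character attaches the actor to it, with no detach logic.
; Input is enabled for player controller 0, so holding O sets a push flag.
; While attached and pushing, Tick sets the Cube component's world location from the parent actor's location, without sweeping.
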(event `self.ReceiveBeginPlay`
  (`self.EnableInput` (`GameplayStatics.GetPlayerController` 0)))

(event `self.Box.OnComponentBeginOverlap`
  (params (OverlappedComponent :type "PrimitiveComponent Object Reference") (OtherActor :type "Actor Object Reference") (OtherComp :type "PrimitiveComponent Object Reference") (OtherBodyIndex :type Integer) (bFromSweep :type Boolean) (SweepResult :type "HitResult Structure (by ref)"))
  (if (not (`self.ActorsAttached`))
    (bind _asthird_person_perspective_switch (cast `/Game/Fruitcake_Game/Character/ThirdPerson_PerspectiveSwitch` OtherActor))
    (`self.K2_AttachToActor` _asthird_person_perspective_switch "None" "KeepRelative" "KeepRelative" "KeepRelative")
    (set `self.ActorsAttached` true)))

(event `Key|O`
  (params (Key :type "Key Structure"))
  (:`Pressed`
    (set `self.objectpush` true))
  (:`Released`
    (set `self.objectpush` false)))

(event `self.ReceiveTick`
  (params (DeltaSeconds :type "Float (single-precision)"))
  (bind _returnvalue (`self.K2_GetActorLocation` (`self.GetAttachParentActor`)))
  (if (`self.ActorsAttached`)
    (if (`self.objectpush`)
      (`SceneComponent.K2_SetWorldLocation` (`self.Cube`) (`KismetMathLibrary.TransformLocation` (`KismetMathLibrary.MakeTransform` _returnvalue) _returnvalue) false false))))

(fn `UserConstructionScript`)