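; Door actor that slides down once its pushed-button count equals ButtonNo, using three attack-triggered buttons placed by transform variables in the construction script.
; Button overlaps call DoorOpening, which checks for the player's active MeleeBox or a PlayerAttack collision profile, then increments the count and turns the button cyan.
; Tick compares the count and drives the door timeline through a FlipFlop until DoorOpened is set.
; The button press animation is never called.
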(event `self.ReceiveTick`
  (params (DeltaSeconds :type "Float (single-precision)"))
  (if (== (`self.buttonNo`) (`self.pushedButons`))
    (if (not (`self.doorOpened`))
      (`/Engine/EditorBlueprintResources/StandardMacros.FlipFlop`
        (:`A`
          (bind (_direction _doortrack) (`Timeline|DoorTimeline` :!label _label)
            (:`Update`
              (`SceneComponent.K2_SetRelativeLocation` (`self.DoorMesh`) (`KismetMathLibrary.VLerp` (0.0 0.0 0.0) (0.0 0.0 -500.0) _doortrack) false false)
              (set `self.doorOpened` true))))
        (:`B`
          (goto _label :!via `Reverse`))))))

(event `self.ButtonCollision.OnComponentBeginOverlap`
  (params (OverlappedComponent :type "PrimitiveComponent Object Reference") (OtherActor :type "Actor Object Reference") (OtherComp :type "PrimitiveComponent Object Reference") (OtherBodyIndex :type Integer) (bFromSweep :type Boolean) (SweepResult :type "HitResult Structure (by ref)"))
  ;[1 1 1] Button Collision Control
  (bind _isopen (`self.DoorOpening` (`self.Button`) (`self.button1Hit`) OtherActor OtherComp))
  (set `self.button1Hit` _isopen))

(event `self.ButtonCollision2.OnComponentBeginOverlap`
  (params (OverlappedComponent :type "PrimitiveComponent Object Reference") (OtherActor :type "Actor Object Reference") (OtherComp :type "PrimitiveComponent Object Reference") (OtherBodyIndex :type Integer) (bFromSweep :type Boolean) (SweepResult :type "HitResult Structure (by ref)"))
  ;[1 1 1] Button Collision Control
  (bind _isopen (`self.DoorOpening` (`self.Button2`) (`self.button3Hit`) OtherActor OtherComp))
  (set `self.button3Hit` _isopen))

(event `self.ButtonCollision1.OnComponentBeginOverlap`
  (params (OverlappedComponent :type "PrimitiveComponent Object Reference") (OtherActor :type "Actor Object Reference") (OtherComp :type "PrimitiveComponent Object Reference") (OtherBodyIndex :type Integer) (bFromSweep :type Boolean) (SweepResult :type "HitResult Structure (by ref)"))
  ;[1 1 1] Button Collision Control
  (bind _isopen (`self.DoorOpening` (`self.Button1`) (`self.button2Hit`) OtherActor OtherComp))
  (set `self.button2Hit` _isopen))

(fn `DoorOpening`
  (params (`Door Mesh` :type "StaticMeshComponent Object Reference") (`Button Bool` :type Boolean) (`Player Object` :type "Object Object Reference") (`Player Component` :type "PrimitiveComponent Object Reference"))
  (returns (IsOpen :type Boolean))
  (bind _asthird_person_perspective_switch (cast `/Game/Fruitcake_Game/Character/ThirdPerson_PerspectiveSwitch` `Player Object`)
    (:`then`
      (if (`PrimitiveComponent.K2_IsQueryCollisionEnabled` (`/Game/Fruitcake_Game/Character/ThirdPerson_PerspectiveSwitch.MeleeBox` _asthird_person_perspective_switch))
        (if `Button Bool`
          (return false)
          (else
            (set `self.pushedButons` (+ (`self.pushedButons`) 1) :!label _label)
            (set `self.Button Bool` false)
            (`PrimitiveComponent.SetMaterial` `Door Mesh` 0 "/Game/Fruitcake_Game/Materials/CyanBloomInstance.CyanBloomInstance")
            (return true)))))
    (:`CastFailed`
      (if (== (`PrimitiveComponent.GetCollisionProfileName` `Player Component`) "PlayerAttack")
        (goto _label)
        (else
          (return false))))))

(fn `UserConstructionScript`
  (`SceneComponent.K2_SetRelativeTransform` (`self.Button`) (`self.ButtonTransform`) false false)
  (`SceneComponent.K2_SetRelativeTransform` (`self.Button1`) (`self.ButtonTransform2`) false false)
  (`SceneComponent.K2_SetRelativeTransform` (`self.Button2`) (`self.ButtonTransform3`) false false))