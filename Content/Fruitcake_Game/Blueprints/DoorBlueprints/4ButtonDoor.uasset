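; Puzzle door that swings open once the player has activated enough of its four buttons.
; Each button registers once, turning green and raising a counter, when ThirdPerson_PerspectiveSwitch overlaps it with MeleeBox query collision enabled.
; Tick compares the counter to ButtonNo and starts a yaw timeline, whose update sets DoorOpened to block retriggering.
; The construction script places buttons from transform variables; the button press animation is never called.
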(event `self.ReceiveTick`
  (params (DeltaSeconds :type "Float (single-precision)"))
  (if (== (`self.buttonNo`) (`self.pushedButons`))
    (if (not (`self.doorOpened`))
      (`/Engine/EditorBlueprintResources/StandardMacros.FlipFlop`
        (:`A`
          (bind (_direction _doortrack) (`Timeline|DoorTimeline` :!label _label)
            (:`Update`
              (`SceneComponent.K2_SetRelativeRotation` (`self.DoorMesh`) (`KismetMathLibrary.MakeRotator` 0.0 0.0 (`KismetMathLibrary.Lerp` (`self.DoorCloseAngle`) (`self.DoorOpenAngle`) _doortrack)) false false)
              (set `self.doorOpened` true))))
        (:`B`
          (goto _label :!via `Reverse`))))))

(event `self.ButtonCollision.OnComponentBeginOverlap`
  (params (OverlappedComponent :type "PrimitiveComponent Object Reference") (OtherActor :type "Actor Object Reference") (OtherComp :type "PrimitiveComponent Object Reference") (OtherBodyIndex :type Integer) (bFromSweep :type Boolean) (SweepResult :type "HitResult Structure (by ref)"))
  (bind _asthird_person_perspective_switch (cast `/Game/Fruitcake_Game/Character/ThirdPerson_PerspectiveSwitch` OtherActor))
  (if (`PrimitiveComponent.K2_IsQueryCollisionEnabled` (`/Game/Fruitcake_Game/Character/ThirdPerson_PerspectiveSwitch.MeleeBox` _asthird_person_perspective_switch))
    (if (not (`self.button1Hit`))
      (set `self.pushedButons` (+ (`self.pushedButons`) 1))
      (set `self.button1Hit` true)
      (`PrimitiveComponent.SetMaterial` (`self.Button`) 0 "/Game/Fruitcake_Game/Materials/Green.Green"))))

(event `self.ButtonCollision1.OnComponentBeginOverlap`
  (params (OverlappedComponent :type "PrimitiveComponent Object Reference") (OtherActor :type "Actor Object Reference") (OtherComp :type "PrimitiveComponent Object Reference") (OtherBodyIndex :type Integer) (bFromSweep :type Boolean) (SweepResult :type "HitResult Structure (by ref)"))
  (bind _asthird_person_perspective_switch (cast `/Game/Fruitcake_Game/Character/ThirdPerson_PerspectiveSwitch` OtherActor))
  (if (`PrimitiveComponent.K2_IsQueryCollisionEnabled` (`/Game/Fruitcake_Game/Character/ThirdPerson_PerspectiveSwitch.MeleeBox` _asthird_person_perspective_switch))
    (if (not (`self.button2Hit`))
      (set `self.pushedButons` (+ (`self.pushedButons`) 1))
      (set `self.button2Hit` true)
      (`PrimitiveComponent.SetMaterial` (`self.Button1`) 0 "/Game/Fruitcake_Game/Materials/Green.Green"))))

(event `self.ButtonCollision2.OnComponentBeginOverlap`
  (params (OverlappedComponent :type "PrimitiveComponent Object Reference") (OtherActor :type "Actor Object Reference") (OtherComp :type "PrimitiveComponent Object Reference") (OtherBodyIndex :type Integer) (bFromSweep :type Boolean) (SweepResult :type "HitResult Structure (by ref)"))
  (bind _asthird_person_perspective_switch (cast `/Game/Fruitcake_Game/Character/ThirdPerson_PerspectiveSwitch` OtherActor))
  (if (`PrimitiveComponent.K2_IsQueryCollisionEnabled` (`/Game/Fruitcake_Game/Character/ThirdPerson_PerspectiveSwitch.MeleeBox` _asthird_person_perspective_switch))
    (if (not (`self.button3Hit`))
      (set `self.pushedButons` (+ (`self.pushedButons`) 1))
      (set `self.button3Hit` true)
      (`PrimitiveComponent.SetMaterial` (`self.Button2`) 0 "/Game/Fruitcake_Game/Materials/Green.Green"))))

(event `self.ButtonCollision3.OnComponentBeginOverlap`
  (params (OverlappedComponent :type "PrimitiveComponent Object Reference") (OtherActor :type "Actor Object Reference") (OtherComp :type "PrimitiveComponent Object Reference") (OtherBodyIndex :type Integer) (bFromSweep :type Boolean) (SweepResult :type "HitResult Structure (by ref)"))
  (bind _asthird_person_perspective_switch (cast `/Game/Fruitcake_Game/Character/ThirdPerson_PerspectiveSwitch` OtherActor))
  (if (`PrimitiveComponent.K2_IsQueryCollisionEnabled` (`/Game/Fruitcake_Game/Character/ThirdPerson_PerspectiveSwitch.MeleeBox` _asthird_person_perspective_switch))
    (if (not (`self.button4Hit`))
      (set `self.pushedButons` (+ (`self.pushedButons`) 1))
      (set `self.button4Hit` true)
      (`PrimitiveComponent.SetMaterial` (`self.Button3`) 0 "/Game/Fruitcake_Game/Materials/Green.Green"))))

(fn `UserConstructionScript`
  (`SceneComponent.K2_SetRelativeTransform` (`self.Button`) (`self.ButtonTransform`) false false)
  (`SceneComponent.K2_SetRelativeTransform` (`self.Button1`) (`self.ButtonTransform2`) false false)
  (`SceneComponent.K2_SetRelativeTransform` (`self.Button2`) (`self.ButtonTransform3`) false false)
  (`SceneComponent.K2_SetRelativeTransform` (`self.Button3`) (`self.ButtonTransform4`) false false))