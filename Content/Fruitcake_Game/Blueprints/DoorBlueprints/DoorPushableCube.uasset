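; DoorPushableCube is a pressure-plate puzzle door that leads to the end-game menu.
; Each plate snaps an overlapping PushableCube onto itself and increments a counter; the first plate requires two presses, while the second triggers regardless.
; A triggered plate plays a timeline macro, then makes the door mesh visible and collidable.
; The player character hitting that mesh shows the end menu and pauses the game.
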(event `self.Plate.OnComponentBeginOverlap`
  (params (OverlappedComponent :type "PrimitiveComponent Object Reference") (OtherActor :type "Actor Object Reference") (OtherComp :type "PrimitiveComponent Object Reference") (OtherBodyIndex :type Integer) (bFromSweep :type Boolean) (SweepResult :type "HitResult Structure (by ref)"))
  (bind _buttons_pressed (`self.Buttons Pressed`))
  ;[1 1 1] Pressure Plate Check
  (bind _aspushable_cube (cast `/Game/Fruitcake_Game/Blueprints/PushCube/PushableCube` OtherActor))
  (set `/Game/Fruitcake_Game/Blueprints/PushCube/PushableCube.OnButton` true _aspushable_cube)
  (`KismetSystemLibrary.MoveComponentTo` (`/Game/Fruitcake_Game/Blueprints/PushCube/PushableCube.StaticMesh` _aspushable_cube) (+ (`SceneComponent.K2_GetComponentLocation` (`self.Plate`)) (0.0 0.0 0.0)) (struct) false false 0.5)
  (set `self.Buttons Pressed` (+ _buttons_pressed 1.0))
  ;[1 1 1] Button and Door Animation
  (if (== _buttons_pressed 2.0)
    (`Timeline|Timeline_0` :!via `PlayFromStart` :!label _label
      (:`Finished`
        (if (not (`self.doorOpened`))
          (`PrimitiveComponent.SetCollisionEnabled` (`self.DoorMesh`) "QueryAndPhysics")
          (`SceneComponent.SetVisibility` (`self.DoorMesh`) true false))))))

(event `self.Plate2.OnComponentBeginOverlap`
  (params (OverlappedComponent :type "PrimitiveComponent Object Reference") (OtherActor :type "Actor Object Reference") (OtherComp :type "PrimitiveComponent Object Reference") (OtherBodyIndex :type Integer) (bFromSweep :type Boolean) (SweepResult :type "HitResult Structure (by ref)"))
  ;[1 1 1] Pressure Plate Check
  (bind _aspushable_cube (cast `/Game/Fruitcake_Game/Blueprints/PushCube/PushableCube` OtherActor))
  (set `/Game/Fruitcake_Game/Blueprints/PushCube/PushableCube.OnButton` true _aspushable_cube)
  (`KismetSystemLibrary.MoveComponentTo` (`/Game/Fruitcake_Game/Blueprints/PushCube/PushableCube.StaticMesh` _aspushable_cube) (+ (`SceneComponent.K2_GetComponentLocation` (`self.Plate2`)) (0.0 0.0 0.0)) (struct) false false 0.5)
  (set `self.Buttons Pressed` (+ (`self.Buttons Pressed`) 1.0))
  (if true
    (goto _label :!via `PlayFromStart`)))

(event `self.DoorMesh.OnComponentHit`
  (params (HitComponent :type "PrimitiveComponent Object Reference") (OtherActor :type "Actor Object Reference") (OtherComp :type "PrimitiveComponent Object Reference") (NormalImpulse :type "Vector Structure") (Hit :type "HitResult Structure (by ref)"))
  (cast `/Game/Fruitcake_Game/Character/ThirdPerson_PerspectiveSwitch` OtherActor)
  (`/Engine/EditorBlueprintResources/StandardMacros.IsValid` (`self.EndMenuRef`)
    (:`Is Valid`
      _)
    (:`Is Not Valid`
      (bind _returnvalue (`|CreateWidget` "/Game/Fruitcake_Game/HUD/MenuUI/EndGameMenuWidget.EndGameMenuWidget_C"))
      (bind _output_get (set `self.EndMenuRef` _returnvalue))))
  (`UserWidget.AddToViewport` _output_get 0)
  (`GameplayStatics.SetGamePaused` true))

(fn `UserConstructionScript`)