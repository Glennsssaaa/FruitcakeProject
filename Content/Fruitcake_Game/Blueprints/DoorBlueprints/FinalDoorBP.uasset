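; Final door that ends the game with a win menu once enough of its four torch objectives are completed.
; Two torches light when hit by the player's melee or attack collision, via the shared DoorOpening function.
; Tick alternates through a FlipFlop to light the others when tagged left or right enemies are gone.
; At the required count, it sets the player's camera speed and door location, waits, then pauses for the menu.
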(event `self.ReceiveTick`
  (params (DeltaSeconds :type "Float (single-precision)"))
  (bind _playerref (`self.playerRef`))
  (if (== (`self.buttonNo`) (`self.pushedButons`))
    (if (not (`self.doorOpened`))
      (set `self.doorOpened` true)
      (set `/Game/Fruitcake_Game/Character/ThirdPerson_PerspectiveSwitch.CameraSpeed` 0.1 _playerref)
      (set `/Game/Fruitcake_Game/Character/ThirdPerson_PerspectiveSwitch.doorLocation` (-2484.091064 5429.77832 5000.0) _playerref)
      (`KismetSystemLibrary.Delay` 6.0)
      (`GameplayStatics.SetGamePaused` true)
      (bind _returnvalue (`|CreateWidget` "/Game/Fruitcake_Game/HUD/MenuUI/WinGameMenuWidget.WinGameMenuWidget_C"))
      (`UserWidget.AddToViewport` _returnvalue 0)
      (set `PlayerController.bShowMouseCursor` true (`GameplayStatics.GetPlayerController` 0)))
    (else
      (`/Engine/EditorBlueprintResources/StandardMacros.FlipFlop`
        (:`A`
          (if (not (`self.button2Hit`))
            (bind _outactors (`GameplayStatics.GetAllActorsOfClassWithTag` "/Game/Fruitcake_Game/Enemies/MushroomJumpEnemy.MushroomJumpEnemy_C" "leftEnemy"))
            (bind _outactors_2 (`GameplayStatics.GetAllActorsOfClassWithTag` "/Game/Fruitcake_Game/Enemies/FlowerEnemy.FlowerEnemy_C" "leftEnemy"))
            (set `self.enemyAmount` (+ (`KismetArrayLibrary.Array_Length` _outactors_2) (`KismetArrayLibrary.Array_Length` _outactors)))
            (if (== (`self.enemyAmount`) 0)
              (set `self.button2Hit` true)
              (`ActorComponent.Activate` (`self.Niagara5`) false)
              (`LightComponent.SetIntensity` (`self.PointLight5`) 10000.0)
              (set `self.pushedButons` (+ (`self.pushedButons`) 1)))))
        (:`B`
          (if (not (`self.button3Hit`))
            (bind _outactors_3 (`GameplayStatics.GetAllActorsOfClassWithTag` "/Game/Fruitcake_Game/Enemies/RadishEnemy.RadishEnemy_C" "rightEnemy"))
            (set `self.enemyAmount2` (`KismetArrayLibrary.Array_Length` _outactors_3))
            (if (== (`self.enemyAmount2`) 0)
              (set `self.button3Hit` true)
              (`ActorComponent.Activate` (`self.Niagara6`) false)
              (`LightComponent.SetIntensity` (`self.PointLight6`) 10000.0)
              (set `self.pushedButons` (+ (`self.pushedButons`) 1)))))))))

(event `self.ButtonCollision.OnComponentBeginOverlap`
  (params (OverlappedComponent :type "PrimitiveComponent Object Reference") (OtherActor :type "Actor Object Reference") (OtherComp :type "PrimitiveComponent Object Reference") (OtherBodyIndex :type Integer) (bFromSweep :type Boolean) (SweepResult :type "HitResult Structure (by ref)"))
  (bind _button1hit (`self.button1Hit`))
  ;[1 1 1] Button Collision Control
  (if (not _button1hit)
    (bind _isopen (`self.DoorOpening` (`self.Torch1`) _button1hit OtherActor OtherComp))
    (bind _output_get (set `self.button1Hit` _isopen))
    (if _output_get
      (`ActorComponent.Activate` (`self.Niagara4`) false)
      (`LightComponent.SetIntensity` (`self.PointLight4`) 10000.0)
      (`AudioComponent.Play` (`self.TorchSound`) 0.0))))

(event `self.ButtonCollision1.OnComponentBeginOverlap`
  (params (OverlappedComponent :type "PrimitiveComponent Object Reference") (OtherActor :type "Actor Object Reference") (OtherComp :type "PrimitiveComponent Object Reference") (OtherBodyIndex :type Integer) (bFromSweep :type Boolean) (SweepResult :type "HitResult Structure (by ref)"))
  ;[1 1 1] Button Collision Control
  (if (not (`self.button4Hit`))
    (bind _isopen (`self.DoorOpening` (`self.Torch2`) false OtherActor OtherComp))
    (bind _output_get (set `self.button4Hit` _isopen))
    (if _output_get
      (`ActorComponent.Activate` (`self.Niagara7`) false)
      (`LightComponent.SetIntensity` (`self.PointLight7`) 10000.0)
      (`AudioComponent.Play` (`self.TorchSound`) 0.0))))

(event `self.ReceiveBeginPlay`
  (bind _outactors (`GameplayStatics.GetAllActorsOfClass` "/Game/Fruitcake_Game/Character/ThirdPerson_PerspectiveSwitch.ThirdPerson_PerspectiveSwitch_C"))
  (set `self.playerRef` (`|GetArrayItem` _outactors))
  (bind _returnvalue (`GameplayStatics.CreateSound2D` "/Game/Fruitcake_Game/Sounds/Torch_Light.Torch_Light" 1.0 1.0 0.0 null false false))
  (set `self.TorchSound` _returnvalue))

(fn `DoorOpening`
  (params (`Door Mesh` :type "StaticMeshComponent Object Reference") (`Button Bool` :type Boolean) (`Player Object` :type "Object Object Reference") (`Player Component` :type "PrimitiveComponent Object Reference"))
  (returns (IsOpen :type Boolean))
  (bind _returnvalue (+ (`self.pushedButons`) 1))
  (bind _asthird_person_perspective_switch (cast `/Game/Fruitcake_Game/Character/ThirdPerson_PerspectiveSwitch` `Player Object`)
    (:`then`
      (if (`PrimitiveComponent.K2_IsQueryCollisionEnabled` (`/Game/Fruitcake_Game/Character/ThirdPerson_PerspectiveSwitch.MeleeBox` _asthird_person_perspective_switch))
        (if `Button Bool`
          (set `self.pushedButons` _returnvalue)
          (return false)
          (else
            (set `self.pushedButons` _returnvalue :!label _label)
            (set `self.Button Bool` false)
            (`PrimitiveComponent.SetMaterial` `Door Mesh` 0 "/Game/Fruitcake_Game/Materials/ButtonsTrim.ButtonsTrim")
            (return true)))))
    (:`CastFailed`
      (if (== (`PrimitiveComponent.GetCollisionProfileName` `Player Component`) "PlayerAttack")
        (goto _label)
        (else
          (return false))))))

(fn `UserConstructionScript`)