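; Pushable-cube puzzle Blueprint where a pressure button swings a door open.
; X and Y trigger volumes lock the matching physics constraint axis and enable cube physics when the perspective-switch player enters, freeing it on exit.
; Any Box1 overlap disables physics, sets OnButton to block further pushing, moves the cube above the button and turns the button green.
; A FlipFlop alternates a timeline forward and backward to rotate the door's yaw.
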(event `self.YCollision.OnComponentEndOverlap`
  (params (OverlappedComponent :type "PrimitiveComponent Object Reference") (OtherActor :type "Actor Object Reference") (OtherComp :type "PrimitiveComponent Object Reference") (OtherBodyIndex :type Integer))
  (`PhysicsConstraintComponent.SetLinearYLimit` (`self.PhysicsConstraint`) "LCM_Free" 0.0))

(event `self.YCollision.OnComponentBeginOverlap`
  (params (OverlappedComponent :type "PrimitiveComponent Object Reference") (OtherActor :type "Actor Object Reference") (OtherComp :type "PrimitiveComponent Object Reference") (OtherBodyIndex :type Integer) (bFromSweep :type Boolean) (SweepResult :type "HitResult Structure (by ref)"))
  (if (not (`self.onButton`))
    (cast `/Game/Fruitcake_Game/Character/ThirdPerson_PerspectiveSwitch` OtherActor)
    (`PhysicsConstraintComponent.SetLinearYLimit` (`self.PhysicsConstraint`) "LCM_Locked" 0.0)
    (`PrimitiveComponent.SetSimulatePhysics` (`self.PushCube`) true)))

(event `self.XCollision.OnComponentEndOverlap`
  (params (OverlappedComponent :type "PrimitiveComponent Object Reference") (OtherActor :type "Actor Object Reference") (OtherComp :type "PrimitiveComponent Object Reference") (OtherBodyIndex :type Integer))
  (`PhysicsConstraintComponent.SetLinearXLimit` (`self.PhysicsConstraint`) "LCM_Free" 0.0))

(event `self.XCollision.OnComponentBeginOverlap`
  (params (OverlappedComponent :type "PrimitiveComponent Object Reference") (OtherActor :type "Actor Object Reference") (OtherComp :type "PrimitiveComponent Object Reference") (OtherBodyIndex :type Integer) (bFromSweep :type Boolean) (SweepResult :type "HitResult Structure (by ref)"))
  (if (not (`self.onButton`))
    (cast `/Game/Fruitcake_Game/Character/ThirdPerson_PerspectiveSwitch` OtherActor)
    (`PhysicsConstraintComponent.SetLinearXLimit` (`self.PhysicsConstraint`) "LCM_Locked" 0.0)
    (`PrimitiveComponent.SetSimulatePhysics` (`self.PushCube`) true)))

(event `self.Box1.OnComponentBeginOverlap`
  (params (OverlappedComponent :type "PrimitiveComponent Object Reference") (OtherActor :type "Actor Object Reference") (OtherComp :type "PrimitiveComponent Object Reference") (OtherBodyIndex :type Integer) (bFromSweep :type Boolean) (SweepResult :type "HitResult Structure (by ref)"))
  (`PrimitiveComponent.SetSimulatePhysics` (`self.PushCube`) false)
  (set `self.onButton` true)
  (`KismetSystemLibrary.MoveComponentTo` (`self.PushCube`) (`KismetMathLibrary.TransformLocation` (`KismetMathLibrary.MakeTransform` (0.0 0.0 65.0)) (`SceneComponent.K2_GetComponentLocation` (`self.Cube`))) (struct) false false 1.0)
  (`PrimitiveComponent.SetMaterial` (`self.Cube`) 0 "/Game/Fruitcake_Game/Materials/Green.Green")
  (`/Engine/EditorBlueprintResources/StandardMacros.FlipFlop`
    (:`A`
      (bind (_direction _doortrack) (`Timeline|Timeline_0` :!label _label)
        (:`Update`
          (`SceneComponent.K2_SetRelativeRotation` (`self.DoorMesh`) (`KismetMathLibrary.MakeRotator` 0.0 0.0 (`KismetMathLibrary.Lerp` (`self.DoorCloseAngle`) (`self.DoorOpenAngle`) _doortrack)) false false))))
    (:`B`
      (goto _label :!via `Reverse`))))

(fn `UserConstructionScript`)