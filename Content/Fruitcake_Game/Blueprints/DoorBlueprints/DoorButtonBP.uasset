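; Torch button that opens its own sliding door when the player hits it with melee or a PlayerAttack-profile component.
; Melee hits count only if the button passes the player's behind-wall check; a DoorOpened flag blocks retriggering.
; A hit swaps the torch material, runs a press macro, then a timeline lowers and hides the door while lighting effects and sounds play.
; Actors tagged camPan also pass their location to the player as DoorLocation.
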(event `self.ButtonCollision.OnComponentBeginOverlap`
  (params (OverlappedComponent :type "PrimitiveComponent Object Reference") (OtherActor :type "Actor Object Reference") (OtherComp :type "PrimitiveComponent Object Reference") (OtherBodyIndex :type Integer) (bFromSweep :type Boolean) (SweepResult :type "HitResult Structure (by ref)"))
  ;[1 1 1] Is Button Colliding with Player Melee or Projectile
  (bind _asthird_person_perspective_switch (cast `/Game/Fruitcake_Game/Character/ThirdPerson_PerspectiveSwitch` OtherActor)
    (:`then`
      (bind _returnvalue (`PlayerCharacter.CheckIfButtonIsBehindWall` _asthird_person_perspective_switch (`self.ButtonCollision`)))
      (if _returnvalue
        _
        (elif (`PrimitiveComponent.K2_IsQueryCollisionEnabled` (`/Game/Fruitcake_Game/Character/ThirdPerson_PerspectiveSwitch.MeleeBox` _asthird_person_perspective_switch))
          (if (not (`self.doorOpened`)) :!label _label
            (`AudioComponent.Play` (`self.Torch Sound`) 0.0)
            (if true
              (if (`self.ActorHasTag` "camPan")
                (set `/Game/Fruitcake_Game/Character/ThirdPerson_PerspectiveSwitch.doorLocation` (`SceneComponent.K2_GetComponentLocation` (`self.DefaultSceneRoot`)) (`self.playerRef`)))
              (set `self.doorOpened` true)
              ;[1 1 1] Button and Door Animation
              (`PrimitiveComponent.SetMaterial` (`self.ButtonTorch`) 0 "/Game/Fruitcake_Game/Materials/ButtonsTrim.ButtonsTrim")
              (`Timeline|Button Press` :!via `PlayFromStart`
                (:`Finished`
                  (`/Engine/EditorBlueprintResources/StandardMacros.FlipFlop`
                    (:`A`
                      (`AudioComponent.Play` (`self.Door Sound`) 0.0)
                      (bind (_direction _doortrack) (`Timeline|DoorTimeline` :!label _label_2)
                        (:`Update`
                          (`SceneComponent.K2_SetRelativeLocation` (`self.DoorMesh`) (`KismetMathLibrary.VLerp` (0.0 0.0 0.0) (0.0 0.0 -500.0) _doortrack) false false)
                          (set `self.doorOpened` true)
                          (`ActorComponent.Activate` (`self.Niagara`) false)
                          (`LightComponent.SetIntensity` (`self.PointLight`) 10000.0)
                          (`ActorComponent.Activate` (`self.Niagara1`) false)
                          (`LightComponent.SetIntensity` (`self.PointLight1`) 10000.0))
                        (:`Finished`
                          (`SceneComponent.SetVisibility` (`self.DoorMesh`) false false))))
                    (:`B`
                      (goto _label_2 :!via `Reverse`))))))))))
    (:`CastFailed`
      (if (== (`PrimitiveComponent.GetCollisionProfileName` OtherComp) "PlayerAttack")
        (goto _label)))))

(event `self.ReceiveBeginPlay`
  (bind _outactors (`GameplayStatics.GetAllActorsOfClass` "/Game/Fruitcake_Game/Character/ThirdPerson_PerspectiveSwitch.ThirdPerson_PerspectiveSwitch_C"))
  (set `self.playerRef` (`|GetArrayItem` _outactors))
  (`StaticMeshComponent.SetStaticMesh` (`self.ButtonTorch`) (`self.buttonMesh`))
  (bind _returnvalue (`GameplayStatics.CreateSound2D` "/Game/Fruitcake_Game/Sounds/Torch_Light.Torch_Light" 1.0 1.0 0.0 null))
  (set `self.Torch Sound` _returnvalue)
  (bind _returnvalue_2 (`GameplayStatics.CreateSound2D` "/Game/Fruitcake_Game/Sounds/Stone_Slide-01.Stone_Slide-01" 1.0 1.0 0.0 null))
  (set `self.Door Sound` _returnvalue_2))

(fn `UserConstructionScript`)