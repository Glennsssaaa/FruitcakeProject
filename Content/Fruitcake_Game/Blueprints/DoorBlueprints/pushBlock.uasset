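; A push block actor that is meant to let the player shove its physics cube.
; Each tick, while the player character's BoxPushing flag is on, Overlapping selects a slowed walk speed with cube physics enabled, or normal speed.
; Ending overlap with YBox clears Overlapping for the player, but the begin-overlap event is empty and the logic setting it true is disconnected.
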(event `self.ReceiveBeginPlay`
  (bind _asthird_person_perspective_switch (cast `/Game/Fruitcake_Game/Character/ThirdPerson_PerspectiveSwitch` (`GameplayStatics.GetPlayerCharacter` 0)))
  (set `self.As Third Person Perspective Switch` _asthird_person_perspective_switch))

(event `self.ReceiveTick`
  (params (DeltaSeconds :type "Float (single-precision)"))
  (bind _as_third_person_perspective_switch (`self.As Third Person Perspective Switch`))
  (if (`/Game/Fruitcake_Game/Character/ThirdPerson_PerspectiveSwitch.boxPushing` _as_third_person_perspective_switch)
    (if (`self.overlapping`)
      (set `CharacterMovementComponent.MaxWalkSpeed` 100.0 (`Character.CharacterMovement` _as_third_person_perspective_switch))
      (`PrimitiveComponent.SetSimulatePhysics` (`self.Cube`) true)
      (else
        (set `CharacterMovementComponent.MaxWalkSpeed` 600.0 (`Character.CharacterMovement` (`self.As Third Person Perspective Switch`)))))))

(event `self.YBox.OnComponentBeginOverlap`
  (params (OverlappedComponent :type "PrimitiveComponent Object Reference") (OtherActor :type "Actor Object Reference") (OtherComp :type "PrimitiveComponent Object Reference") (OtherBodyIndex :type Integer) (bFromSweep :type Boolean) (SweepResult :type "HitResult Structure (by ref)")))

(event `self.YBox.OnComponentEndOverlap`
  (params (OverlappedComponent :type "PrimitiveComponent Object Reference") (OtherActor :type "Actor Object Reference") (OtherComp :type "PrimitiveComponent Object Reference") (OtherBodyIndex :type Integer))
  (if (== null (`self.As Third Person Perspective Switch`))
    (set `self.overlapping` false)))

(fn `UserConstructionScript`)