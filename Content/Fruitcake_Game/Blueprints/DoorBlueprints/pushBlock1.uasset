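; Pushable block actor for the perspective-switch third-person character, apparently unfinished.
; Caches the player on BeginPlay, then enables that character's input when anything begins overlapping YBox and disables it on exit.
; On exit during BoxPushing, the Cube stops simulating physics and detaches.
; Tick's FlipFlop attach/detach sits behind an always-false condition, and the walk-speed and physics push logic is unconnected.
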(event `self.ReceiveBeginPlay`
  (bind _asthird_person_perspective_switch (cast `/Game/Fruitcake_Game/Character/ThirdPerson_PerspectiveSwitch` (`GameplayStatics.GetPlayerCharacter` 0)))
  (set `self.As Third Person Perspective Switch` _asthird_person_perspective_switch))

(event `self.YBox.OnComponentBeginOverlap`
  (params (OverlappedComponent :type "PrimitiveComponent Object Reference") (OtherActor :type "Actor Object Reference") (OtherComp :type "PrimitiveComponent Object Reference") (OtherBodyIndex :type Integer) (bFromSweep :type Boolean) (SweepResult :type "HitResult Structure (by ref)"))
  (`self.EnableInput` (`self.As Third Person Perspective Switch`) (`GameplayStatics.GetPlayerController` 0)))

(event `self.YBox.OnComponentEndOverlap`
  (params (OverlappedComponent :type "PrimitiveComponent Object Reference") (OtherActor :type "Actor Object Reference") (OtherComp :type "PrimitiveComponent Object Reference") (OtherBodyIndex :type Integer))
  (bind _as_third_person_perspective_switch (`self.As Third Person Perspective Switch`))
  (bind _cube (`self.Cube`))
  (`self.DisableInput` _as_third_person_perspective_switch (`GameplayStatics.GetPlayerController` 0))
  (if (`/Game/Fruitcake_Game/Character/ThirdPerson_PerspectiveSwitch.boxPushing` _as_third_person_perspective_switch)
    (`PrimitiveComponent.SetSimulatePhysics` _cube false)
    (`SceneComponent.K2_DetachFromComponent` _cube "KeepRelative" "KeepRelative" "KeepRelative" true)))

(event `self.ReceiveTick`
  (params (DeltaSeconds :type "Float (single-precision)"))
  (bind _movingobject (`self.MovingObject`))
  (bind _playerref (`self.PlayerRef`))
  (if (or false false)
    (bind _isa (`/Engine/EditorBlueprintResources/StandardMacros.FlipFlop`)
      (:`A`
        (set `self.IsAPressed?` _isa)
        (set `/Game/Fruitcake_Game/Blueprints/DoorBlueprints/pushBlock1.IsPushingObject` true _playerref)
        (`PrimitiveComponent.SetSimulatePhysics` _movingobject true)
        (`SceneComponent.K2_AttachToComponent` _movingobject (`Character.Mesh` _playerref) "None" "KeepWorld" "KeepRelative" "KeepRelative" true))
      (:`B`
        (set `/Game/Fruitcake_Game/Blueprints/DoorBlueprints/pushBlock1.IsPushingObject` false _playerref)
        (`PrimitiveComponent.SetSimulatePhysics` _movingobject false)
        (`SceneComponent.K2_DetachFromComponent` _movingobject "KeepWorld" "KeepRelative" "KeepRelative" true)))))

(fn `UserConstructionScript`)