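; BP_Volumetrics builds a layered volume effect at BeginPlay by stacking static mesh components vertically above a base Plane.
; VolumeResolution drives the number of collision-free layers, spaced by VolumeHeight divided by that resolution.
; The base Plane and each layer get a dynamic material instance fed the Plane's world Z and VolumeHeight as MinFrom_BP and MaxFrom_BP, so the material receives the volume's vertical parameters.
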(event `self.ReceiveBeginPlay`
  (bind _plane (`self.Plane`))
  (bind (_returnvalue_x _returnvalue_y _returnvalue_z) (`KismetMathLibrary.BreakVector` (`SceneComponent.K2_GetComponentLocation` _plane)))
  (bind _returnvalue (+ (`self.PreviousLayerHeight`) (/ (`self.VolumeHeight`) (`KismetMathLibrary.Conv_IntToDouble` (`self.VolumeResolution`)))))
  (bind _returnvalue_2 (`PrimitiveComponent.CreateDynamicMaterialInstance` _plane 0 (`PrimitiveComponent.GetMaterial` _plane 0) "None"))
  (bind _output_get (set `self.SeedHeight` _returnvalue_z))
  (`MaterialInstanceDynamic.SetScalarParameterValue` _returnvalue_2 "MinFrom_BP" _output_get)
  (`MaterialInstanceDynamic.SetScalarParameterValue` _returnvalue_2 "MaxFrom_BP" (`self.VolumeHeight`))
  (for _ (range (+ (`self.VolumeResolution`) 1))
    (bind _returnvalue_3 (`AddComponent|NODE_AddStaticMeshComponent-0` :`RelativeTransform` (`KismetMathLibrary.MakeTransform` (`KismetMathLibrary.MakeVector` 0.0 0.0 _returnvalue))))
    (`PrimitiveComponent.SetCollisionEnabled` _returnvalue_3 "NoCollision")
    (set `self.PreviousLayerHeight` _returnvalue)
    (bind _returnvalue_4 (`PrimitiveComponent.CreateDynamicMaterialInstance` _returnvalue_3 0 (`PrimitiveComponent.GetMaterial` _returnvalue_3 0) "None"))
    (`MaterialInstanceDynamic.SetScalarParameterValue` _returnvalue_4 "MinFrom_BP" (`self.SeedHeight`))
    (`MaterialInstanceDynamic.SetScalarParameterValue` _returnvalue_4 "MaxFrom_BP" (`self.VolumeHeight`))))

(fn `UserConstructionScript`)