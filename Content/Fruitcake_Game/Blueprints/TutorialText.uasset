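; TutorialText is a one-shot trigger that shows tutorial text on screen when the ThirdPerson_PerspectiveSwitch actor enters its Box.
; On first overlap it sets the Entered flag, creates a TutorialWidget and adds it to the viewport.
; Two timelines, separated by a short hold, feed opacity and the two text variables to the widget through GetText.
; The widget is removed when the second timeline finishes, and Entered stays set to prevent repeats.
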(event `self.Box.OnComponentBeginOverlap`
  (params (OverlappedComponent :type "PrimitiveComponent Object Reference") (OtherActor :type "Actor Object Reference") (OtherComp :type "PrimitiveComponent Object Reference") (OtherBodyIndex :type Integer) (bFromSweep :type Boolean) (SweepResult :type "HitResult Structure (by ref)"))
  (bind _tutorialtext2 (`self.TutorialText2`))
  (bind _tutorialtext (`self.TutorialText`))
  (if (not (`self.Entered`))
    (cast `/Game/Fruitcake_Game/Character/ThirdPerson_PerspectiveSwitch` OtherActor)
    (set `self.Entered` true)
    (bind _returnvalue (`|CreateWidget` "/Game/Fruitcake_Game/HUD/TutorialWidget.TutorialWidget_C"))
    (`UserWidget.AddToViewport` _returnvalue 0)
    (bind (_direction _newtrack_0) (`Timeline|Timeline_0` :!via `PlayFromStart`)
      (:`Update`
        (`/Game/Fruitcake_Game/HUD/TutorialWidget.getText` _returnvalue _tutorialtext _newtrack_0 _tutorialtext2))
      (:`Finished`
        (`KismetSystemLibrary.Delay` 4.0)
        (bind (_direction_2 _newtrack_0_2) (`Timeline|Timeline_1` :!via `PlayFromStart`)
          (:`Update`
            (`/Game/Fruitcake_Game/HUD/TutorialWidget.getText` _returnvalue _tutorialtext _newtrack_0_2 _tutorialtext2))
          (:`Finished`
            (`Widget.RemoveFromParent` _returnvalue)
            (set `self.Entered` true)))))))

(fn `UserConstructionScript`)