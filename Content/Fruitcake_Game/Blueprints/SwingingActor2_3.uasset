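; Actor with two physics-constrained swings, Swing and Swing1, that it keeps pushing to sustain their motion.
; BeginPlay sets their starting world rotations with opposite-signed 180-degree angles.
; Tick uses a FlipFlop to service one swing per frame, reading its constraint's angular Y force and the swing's pitch.
; When both pass their threshold checks, it overrides that swing's linear velocity with a fixed negative-Y push.
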(event `self.ReceiveBeginPlay`
  (`SceneComponent.K2_SetWorldRotation` (`self.Swing`) (struct :`Roll` -180.0) false false)
  (`SceneComponent.K2_SetWorldRotation` (`self.Swing1`) (struct :`Roll` 180.0) false false))

(event `self.ReceiveTick`
  (params (DeltaSeconds :type "Float (single-precision)"))
  (bind (_returnvalue_roll _returnvalue_pitch) (`KismetMathLibrary.BreakRotator` (`SceneComponent.K2_GetComponentRotation` (`self.Swing1`))))
  (bind (_returnvalue_roll_2 _returnvalue_pitch_2) (`KismetMathLibrary.BreakRotator` (`SceneComponent.K2_GetComponentRotation` (`self.Swing`))))
  (`/Engine/EditorBlueprintResources/StandardMacros.FlipFlop`
    (:`A`
      (bind (_outlinearforce _outangularforce) (`PhysicsConstraintComponent.GetConstraintForce` (`self.PhysicsConstraint`)))
      (if (> (.y _outangularforce) -4000.0)
        (if (< _returnvalue_pitch_2 0.8)
          (`PrimitiveComponent.SetPhysicsLinearVelocity` (`self.Swing`) (0.0 -1200.0 0.0) false "None"))))
    (:`B`
      (bind (_outlinearforce_2 _outangularforce_2) (`PhysicsConstraintComponent.GetConstraintForce` (`self.PhysicsConstraint1`)))
      (if (> (.y _outangularforce_2) -4000.0)
        (if (< _returnvalue_pitch 0.9)
          (`PrimitiveComponent.SetPhysicsLinearVelocity` (`self.Swing1`) (0.0 -1250.0 0.0) false "None"))))))

(fn `UserConstructionScript`)