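; SwingingActor is a physics-driven swing that hangs on a constraint and re-pushes itself as it moves.
; On BeginPlay it sets the Swing component to a steep starting pitch.
; Each Tick, when the PhysicsConstraint's angular Y force is above a threshold and the Swing's world pitch is high enough, it overwrites the Swing's linear velocity with a fixed push along negative Y.
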(event `self.ReceiveBeginPlay`
  (`SceneComponent.K2_SetWorldRotation` (`self.Swing`) (struct :`Roll` 80.0) false false))

(event `self.ReceiveTick`
  (params (DeltaSeconds :type "Float (single-precision)"))
  (bind (_returnvalue_roll _returnvalue_pitch) (`KismetMathLibrary.BreakRotator` (`SceneComponent.K2_GetComponentRotation` (`self.Swing`))))
  (bind (_outlinearforce _outangularforce) (`PhysicsConstraintComponent.GetConstraintForce` (`self.PhysicsConstraint`)))
  (if (> (.y _outangularforce) -4000.0)
    (if (> _returnvalue_pitch 67.0)
      (`PrimitiveComponent.SetPhysicsLinearVelocity` (`self.Swing`) (0.0 -1000.0 0.0) false "None"))))

(fn `UserConstructionScript`)